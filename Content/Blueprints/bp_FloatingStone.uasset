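; Floating stone actor that travels along the spline of a lava path in the level.
; On BeginPlay it finds the Bp_LavaPath actor, caches its spline length and plays a timeline.
; Each timeline update maps the alpha to a distance along the spline and moves the stone to that world location without sweeping.
; The transform is built from location alone, so the spline's rotation is not followed.
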(event `self.ReceiveBeginPlay`
  ;[1 1 1] Start path on begin play
  (bind _returnvalue (`GameplayStatics.GetActorOfClass` "/Game/Blueprints/bp_LavaPath.bp_LavaPath_C"))
  (set `self.PathReference` _returnvalue)
  (set `self.PathLength` (`SplineComponent.GetSplineLength` (`/Game/Blueprints/bp_LavaPath.Spline` (`self.PathReference`))))
  (`self.PlayPathTimeline`))

(event `PlayPathTimeline`
  (bind (_direction _lavapathmovement) (`Timeline|LavaPathTimeline`)
    (:`Update`
      (`self.K2_SetActorTransform` (`KismetMathLibrary.Conv_VectorToTransform` (`SplineComponent.GetLocationAtDistanceAlongSpline` (`/Game/Blueprints/bp_LavaPath.Spline` (`self.PathReference`)) (`KismetMathLibrary.Lerp` 0.0 (`self.PathLength`) _lavapathmovement) "World"))))))

(fn `UserConstructionScript`)